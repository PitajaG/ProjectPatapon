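; Player carriage that carries attached drums and obeys March and Defend commands from the rhythm manager.
; March runs a timeline that advances it along a spline road, snapping it to the ground by downward trace and spinning the wheels.
; Defend opens a brief deflect window within a longer block; DefendBox deflects or absorbs projectiles implementing BPI_DeflectableProjectile.
; HurtBox hits damage the health component, and death opens the death screen level.
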(event `self.ReceiveBeginPlay`
  ; Adding wheels to array
  (set `self.Wheels` (`|MakeArray` (`self.Wheel_1`) (`self.Wheel_2`) (`self.Wheel_3`) (`self.Wheel_4`)))
  ; Attach drums to carriage
  (for _array_element (`self.AttachedDrums`)
    (`self.K2_AttachToActor` _array_element self "None" "KeepWorld" "KeepWorld" "KeepWorld" true)
    ; Set rythm manager reference and bind event to OnCommandIssued function
    (bind _returnvalue (`GameplayStatics.GetActorOfClass` "/Game/Prototype/Blueprints/Rythm_manager_BP.Rythm_manager_BP_C"))
    (bind _output_get (set `self.RythmManagerRef` _returnvalue))
    (add `/Game/Prototype/Blueprints/Rythm_manager_BP.OnCommandIssued` _output_get (delegate `ListenToCommand`))))

(event `ListenToCommand`
  (params (Command :type "/Game/Prototype/Enums/E_CommandType Enum" :default "NewEnumerator0"))
  (bind _spline (`/Game/Prototype/Blueprints/BP_Path.Spline` (`self.SplineRef`)))
  ; Set rythm manager reference and bind event to OnCommandIssued function
  (switch `/Game/Prototype/Enums/E_CommandType` Command
    (:`NewEnumerator2`
      ; Carriage movement on command
      ;; Setting current distance and target distance
      (set `self.CurrentDistance` (`self.LiveDistance`))
      (set `self.TargetDistance` (+ (`self.CurrentDistance`) (* (`self.StepLength`) (`self.MoveSpeed`))))
      (bind (_direction _newtrack_0) (`Timeline|MarchTimeline` :!via `PlayFromStart`)
        (:`Update`
          (`self.RotateWheels` -2.0)
          ;; Getting location and rotation along spline road
          (bind _output_get (set `self.LiveDistance` (`KismetMathLibrary.Lerp` (`self.CurrentDistance`) (`self.TargetDistance`) _newtrack_0)))
          (bind _output_get_2 (set `self.SplinePos` (`SplineComponent.GetLocationAtDistanceAlongSpline` _spline _output_get "World")))
          ;; Getting the ground position by raycast and placing carriage slightly above it
          (bind (_outhit _returnvalue) (`KismetSystemLibrary.LineTraceSingle` _output_get_2 (- _output_get_2 (0.0 0.0 100000.0)) "TraceTypeQuery1"))
          (if _returnvalue
            (`self.K2_SetActorLocationAndRotation` (+ (`.ImpactPoint` (`GameplayStatics.BreakHitResult` _outhit)) (0.0 0.0 75.0)) (`SplineComponent.GetRotationAtDistanceAlongSpline` _spline _output_get "World"))))))
    (:`NewEnumerator3`
      ; Defensive stance
      (set `self.IsDefending` true)
      (set `self.IsInDeflectWindow` true)
      (`KismetSystemLibrary.Delay` (`self.DeflectWindowTime`))
      (set `self.IsInDeflectWindow` false)
      (`KismetSystemLibrary.Delay` 1.0)
      (set `self.IsDefending` false))))

(event `self.DefendBox.OnComponentBeginOverlap`
  (params (OverlappedComponent :type "PrimitiveComponent Object Reference") (OtherActor :type "Actor Object Reference") (OtherComp :type "PrimitiveComponent Object Reference") (OtherBodyIndex :type Integer) (bFromSweep :type Boolean) (SweepResult :type "HitResult Structure (by ref)"))
  ; Defend and deflect trigger
  (if (`KismetSystemLibrary.DoesImplementInterface` OtherActor "/Game/Prototype/Interfaces/BPI_DeflectableProjectile.BPI_DeflectableProjectile_C")
    (if (`self.IsDefending`)
      (if (`self.IsInDeflectWindow`)
        (message `/Game/Prototype/Interfaces/BPI_DeflectableProjectile.OnProjectileDeflect` OtherActor)
        (else
          (message `/Game/Prototype/Interfaces/BPI_DeflectableProjectile.OnProjectileHit` OtherActor))))))

(event `self.HurtBox.OnComponentBeginOverlap`
  (params (OverlappedComponent :type "PrimitiveComponent Object Reference") (OtherActor :type "Actor Object Reference") (OtherComp :type "PrimitiveComponent Object Reference") (OtherBodyIndex :type Integer) (bFromSweep :type Boolean) (SweepResult :type "HitResult Structure (by ref)"))
  ; Getting damage
  (if (`KismetSystemLibrary.DoesImplementInterface` OtherActor "/Game/Prototype/Interfaces/BPI_DeflectableProjectile.BPI_DeflectableProjectile_C")
    (`/Game/Prototype/Blueprints/BPC/BPC_HealthComponent.TakeDamage` (`self.BPC_HealthComponent`) 25.0)
    (message `/Game/Prototype/Interfaces/BPI_DeflectableProjectile.OnProjectileHit` OtherActor)))

(event `/Game/Prototype/Interfaces/BPI_Killable.OnDeath`
  ; On death
  (`GameplayStatics.OpenLevel` "L_DeathScreen"))

(fn `RotateWheels`
  (params (Rotation :type "Float (double-precision)"))
  (for _array_element (`self.Wheels`)
    (`SceneComponent.K2_AddLocalRotation` _array_element (`KismetMathLibrary.MakeRotator` 0.0 Rotation) false false)))

(fn `UserConstructionScript`)