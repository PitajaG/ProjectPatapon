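; Non-VR prototype drum that the player hits with a keyboard key as part of a rhythm mechanic.
; Tick polls the key, and a press plays the drum's FMOD event at the actor and briefly flashes its dynamic material via FlashStrength.
; The press also asks the Rythm_manager_BP found at BeginPlay to check timing, registering this drum's type only when the check passes.
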(event `self.ReceiveBeginPlay`
  (bind _returnvalue (`PrimitiveComponent.CreateDynamicMaterialInstance` (`self.DrumMesh`) 0 (`self.StaticMaterial`) "None"))
  (set `self.DynamicMaterial` _returnvalue)
  (bind _returnvalue_2 (`GameplayStatics.GetActorOfClass` "/Game/Prototype/Blueprints/Rythm_manager_BP.Rythm_manager_BP_C"))
  (set `self.RythmManagerRef` _returnvalue_2))

(event `self.ReceiveTick`
  (params (DeltaSeconds :type "Float (single-precision)"))
  (if (`PlayerController.WasInputKeyJustPressed` (`GameplayStatics.GetPlayerController` 0) (`self.Keyboard_Key`))
    (`|ExecutionSequence`
      (:`then_0`
        (`FMODBlueprintStatics.PlayEventAtLocation` (`self.DrumFmodEvent`) (`KismetMathLibrary.Conv_VectorToTransform` (`self.K2_GetActorLocation`)))
        (`MaterialInstanceDynamic.SetScalarParameterValue` (`self.DynamicMaterial`) "FlashStrength" 10.0 :!label _label)
        (`KismetSystemLibrary.Delay` 0.2)
        (`MaterialInstanceDynamic.SetScalarParameterValue` (`self.DynamicMaterial`) "FlashStrength" 0.0))
      (:`then_1`
        (goto _label))
      (:`then_2`
        (bind _isonbeat (`/Game/Prototype/Blueprints/Rythm_manager_BP.CheckRythmAccuracy` (`self.RythmManagerRef`)))
        (if _isonbeat
          (`/Game/Prototype/Blueprints/Rythm_manager_BP.RegisterDrumHit` (`self.RythmManagerRef`) (`self.MyDrumType`)))))))

(fn `UserConstructionScript`)