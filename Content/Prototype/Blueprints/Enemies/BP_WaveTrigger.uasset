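; BP_WaveTrigger is a one-shot trigger that spawns a wave of melee and ranged enemies when the BP_Carriage overlaps it.
; Spawn points come from the BP_Path spline at set distances ahead of the carriage's LiveDistance, with line traces finding the ground.
; Melee enemies form a row across the path, while ranged enemies alternate between left and right roadside offsets, raised above the ground.
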(event `self.Wave Trigger.OnComponentBeginOverlap`
  (params (OverlappedComponent :type "PrimitiveComponent Object Reference") (OtherActor :type "Actor Object Reference") (OtherComp :type "PrimitiveComponent Object Reference") (OtherBodyIndex :type Integer) (bFromSweep :type Boolean) (SweepResult :type "HitResult Structure (by ref)"))
  (bind _returnvalue (+ (`/Game/Prototype/Blueprints/BP_Carriage.LiveDistance` (`self.WaveCarriageRef`)) (`self.MeleeSpawnDistance`)))
  (bind _returnvalue_2 (+ (`/Game/Prototype/Blueprints/BP_Carriage.LiveDistance` (`self.WaveCarriageRef`)) (`self.RangedSpawnDistance`)))
  (bind _returnvalue_3 (`SplineComponent.GetLocationAtDistanceAlongSpline` (`/Game/Prototype/Blueprints/BP_Path.Spline` (`self.SplineRef`)) _returnvalue "World"))
  ;[0.15 0.1314 0.04635 0.5 72] Spawning ranged mobs
  (bind _asbp_carriage (cast `/Game/Prototype/Blueprints/BP_Carriage` OtherActor))
  (set `self.WaveCarriageRef` _asbp_carriage)
  ;; So the wave doesnt trigger multiple times
  (`/Engine/EditorBlueprintResources/StandardMacros.DoOnce` false
    (:`Completed`
      (`|ExecutionSequence`
        (:`then_0`
          ;[0.15 0.02344 0.02344 0.5 72] Spawning melee mobs
          ;; Getting the ground position by raycast and placing mobs slightly above it
          (bind _outhit (`KismetSystemLibrary.LineTraceSingle` _returnvalue_3 (- _returnvalue_3 (0.0 0.0 100000.0)) "TraceTypeQuery1"))
          (for _index (range 1 (+ (`self.MeleeCount`) 1))
            (`|SpawnActorFromClass` (`self.MeleeEnemyClass`) (`KismetMathLibrary.MakeTransform` (+ (+ (`.ImpactPoint` (`GameplayStatics.BreakHitResult` _outhit)) (0.0 0.0 75.0)) (* (`SplineComponent.GetRightVectorAtDistanceAlongSpline` (`/Game/Prototype/Blueprints/BP_Path.Spline` (`self.SplineRef`)) _returnvalue "World") (* (- _index (/ (+ (`self.MeleeCount`) 1) 2)) 200.0)) (0.0 0.0 0.0)) (`KismetMathLibrary.ComposeRotators` (`SplineComponent.GetRotationAtDistanceAlongSpline` (`/Game/Prototype/Blueprints/BP_Path.Spline` (`self.SplineRef`)) _returnvalue "World") (struct :`Yaw` 180.0))) "AdjustIfPossibleButAlwaysSpawn" "MultiplyWithRoot" null null)))
        (:`then_1`
          (for _index_2 (range 1 (+ (`self.RangedCount`) 1))
            (bind _returnvalue_4 (+ (`SplineComponent.GetLocationAtDistanceAlongSpline` (`/Game/Prototype/Blueprints/BP_Path.Spline` (`self.SplineRef`)) _returnvalue_2 "World") (* (`SplineComponent.GetRightVectorAtDistanceAlongSpline` (`/Game/Prototype/Blueprints/BP_Path.Spline` (`self.SplineRef`)) _returnvalue_2 "World") (`KismetMathLibrary.SelectFloat` (`self.RangedRoadOffset`) (* (`self.RangedRoadOffset`) -1.0) (== (mod _index_2 2) 0)))))
            ;; Getting the ground position by raycast and placing mobs slightly above it
            (bind _outhit_2 (`KismetSystemLibrary.LineTraceSingle` _returnvalue_4 (- _returnvalue_4 (0.0 0.0 100000.0)) "TraceTypeQuery1"))
            (`|SpawnActorFromClass` (`self.RangedEnemyClass`) (`KismetMathLibrary.MakeTransform` (+ (`.ImpactPoint` (`GameplayStatics.BreakHitResult` _outhit_2)) (0.0 0.0 200.0)) (`KismetMathLibrary.ComposeRotators` (`SplineComponent.GetRotationAtDistanceAlongSpline` (`/Game/Prototype/Blueprints/BP_Path.Spline` (`self.SplineRef`)) _returnvalue_2 "World") (struct :`Yaw` 180.0))) "AdjustIfPossibleButAlwaysSpawn" "MultiplyWithRoot" null null)))))))

(event `self.ReceiveBeginPlay`
  ; Setting References
  (bind _returnvalue (`GameplayStatics.GetActorOfClass` "/Game/Prototype/Blueprints/BP_Path.BP_Path_C"))
  (set `self.SplineRef` _returnvalue))

(fn `UserConstructionScript`)