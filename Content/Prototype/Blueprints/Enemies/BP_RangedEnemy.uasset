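; Prototype ranged enemy that fires arrows at the player's carriage in time with the rhythm manager's beat.
; Carriage entering the detection zone activates it and binds it to the beat signal.
; While in range, each beat brightens a dynamic material indicator, and every fourth spawns BP_Arrow aimed at the carriage as placeholder attack logic.
; A separate ApplyDamage function damages carriages in the hitbox, but nothing here calls it.
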(event `self.ReceiveBeginPlay`
  ; Set Rythm Manager Reference
  (bind _returnvalue (`GameplayStatics.GetActorOfClass` "/Game/Prototype/Blueprints/Rythm_manager_BP.Rythm_manager_BP_C"))
  (set `self.RythmManagerRef` _returnvalue))

(event `self.DetectionZone.OnComponentBeginOverlap`
  (params (OverlappedComponent :type "PrimitiveComponent Object Reference") (OtherActor :type "Actor Object Reference") (OtherComp :type "PrimitiveComponent Object Reference") (OtherBodyIndex :type Integer) (bFromSweep :type Boolean) (SweepResult :type "HitResult Structure (by ref)"))
  ; If player in detection range, activate
  (bind _asbp_carriage (castclass `/Game/Prototype/Blueprints/Player/BP_Carriage` (`GameplayStatics.GetObjectClass` OtherActor)))
  (if (== (`GameplayStatics.GetObjectClass` OtherActor) _asbp_carriage)
    (set `self.Carriage Ref` OtherActor)
    (bind _output_get (set `self.IsActive` true))
    ; Connecting event to Beat Signal
    (add `/Game/Prototype/Blueprints/Rythm_manager_BP.Beat Signal` (`self.RythmManagerRef`) (delegate `MoveOnBeat`))))

(event `MoveOnBeat`
  ; Connecting event to Beat Signal
  (set `self.PlayerInAttackRange` (<= (`self.GetDistanceTo` (`self.Carriage Ref`) null) (`self.MaxDistance`)))
  (if (stale `self.DetectionZone.OnComponentBeginOverlap` _output_get)
    (if (`self.PlayerInAttackRange`)
      ; Placeholder attack logic
      (bind _output_get (set `self.AttackCouter` (+ (`self.AttackCouter`) 1)))
      (switch `int` _output_get
        (:`1`
          ;; Increasing brightness each beat signal
          (bind _output_get_2 (set `self.FlashValue` 0.1))
          (`MaterialInstanceDynamic.SetScalarParameterValue` (`self.Dynamicmaterial`) "FlashValue" _output_get_2 :!label _label))
        (:`2`
          (set `self.FlashValue` 0.5)
          (goto _label))
        (:`3`
          (set `self.FlashValue` 10.0)
          (goto _label))
        (:`4`
          (bind _output_get_3 (set `self.FlashValue` 50.0))
          (`MaterialInstanceDynamic.SetScalarParameterValue` (`self.Dynamicmaterial`) "FlashValue" _output_get_3)
          (`|SpawnActorFromClass` "/Game/Prototype/Blueprints/Enemies/BP_Arrow.BP_Arrow_C" (`KismetMathLibrary.MakeTransform` (`self.K2_GetActorLocation`) (`KismetMathLibrary.FindLookAtRotation` (`self.K2_GetActorLocation`) (`self.K2_GetActorLocation` (`self.Carriage Ref`)))) "Undefined" "MultiplyWithRoot" null null)
          (set `self.AttackCouter` 0))))))

(fn `ApplyDamage`
  (for _array_element (`PrimitiveComponent.GetOverlappingActors` (`self.HitBox`) "/Game/Prototype/Blueprints/Player/BP_Carriage.BP_Carriage_C")
    (`/Game/Prototype/Blueprints/BPC/BPC_HealthComponent.TakeDamage` (`self.GetComponentByClass` _array_element "/Game/Prototype/Blueprints/BPC/BPC_HealthComponent.BPC_HealthComponent_C") 25.0)))

(fn `UserConstructionScript`
  (bind _returnvalue (`PrimitiveComponent.CreateDynamicMaterialInstance` (`self.Mesh`) 1 "/Game/Prototype/Materials/M_MobIndicator.M_MobIndicator" "None"))
  (set `self.DynamicMaterial` _returnvalue))