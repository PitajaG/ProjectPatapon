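; Prototype boss enemy that launches a random attack in time with the music.
; It binds to the rhythm manager's beat signal and counts beats, printing a placeholder warning before triggering an attack and resetting the count.
; Each attack spawns either a pair of ranged enemies, one enemy at the melee point (currently also the ranged class), or a boulder.
; The carriage reference and Attacking flag are set but not read here.
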(event `self.ReceiveBeginPlay`
  ; Setting references
  (bind _returnvalue (`GameplayStatics.GetActorOfClass` "/Game/Prototype/Blueprints/Rythm_manager_BP.Rythm_manager_BP_C"))
  (set `self.RythmManagerRef` _returnvalue)
  (bind _returnvalue_2 (`GameplayStatics.GetActorOfClass` "/Game/Prototype/Blueprints/Player/BP_Carriage.BP_Carriage_C"))
  (set `self.CarriageRef` _returnvalue_2)
  ; Connecting boss logic to beat signal
  (add `/Game/Prototype/Blueprints/Rythm_manager_BP.Beat Signal` (`self.RythmManagerRef`) (delegate `BeatSignal`)))

(event `BeatSignal`
  ; Connecting boss logic to beat signal
  ; BeatCounter
  (`|ExecutionSequence`
    (:`then_0`
      (set `self.BeatCounter` (+ (`self.BeatCounter`) 1)))
    (:`then_1`
      (if (== (`self.BeatCounter`) 6)
        ; Incoming attack indicator
        (`KismetSystemLibrary.PrintString` "Hello")
        (else
          ; Calling attack sequence
          (if (>= (`self.BeatCounter`) 8)
            (`self.AttackSequence`)
            (set `self.Attacking` true)
            (set `self.BeatCounter` 0)))))))

(event `AttackSequence`
  ; Attack loop logic
  (bind _output_get (set `self.AttackNumber` (`KismetMathLibrary.RandomIntegerInRange` 0 2)))
  (switch `int` _output_get
    (:`0`
      ;; Spawning ranged oponents
      (`|SpawnActorFromClass` "/Game/Prototype/Blueprints/Enemies/BP_RangedEnemy.BP_RangedEnemy_C" (`self.GetTransform` (`self.LeftRangeSpawnPoint`)) "AdjustIfPossibleButAlwaysSpawn" "MultiplyWithRoot" null null)
      (`|SpawnActorFromClass` "/Game/Prototype/Blueprints/Enemies/BP_RangedEnemy.BP_RangedEnemy_C" (`self.GetTransform` (`self.RightRangeSpawnPoint`)) "AdjustIfPossibleButAlwaysSpawn" "MultiplyWithRoot" null null))
    (:`1`
      ;; Spawning melee oponents
      (`|SpawnActorFromClass` "/Game/Prototype/Blueprints/Enemies/BP_RangedEnemy.BP_RangedEnemy_C" (`self.GetTransform` (`self.MeleeSpawnPoint`)) "AdjustIfPossibleButAlwaysSpawn" "MultiplyWithRoot" null null))
    (:`2`
      ;; Throwing boulder
      (`|SpawnActorFromClass` "/Game/Prototype/Blueprints/BP_Boulder.BP_Boulder_C" (`SceneComponent.K2_GetComponentToWorld` (`self.BoulderSpawn`)) "Undefined" "MultiplyWithRoot" null (`SceneComponent.K2_GetComponentLocation` (`self.BoulderSpawn`)) 5.0 120.0 false null))))

(fn `UserConstructionScript`)