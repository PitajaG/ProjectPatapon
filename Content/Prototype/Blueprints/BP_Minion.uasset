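; BP_Minion is a prototype minion that responds to commands issued by the rhythm manager.
; On BeginPlay it finds the Rythm_manager_BP actor and binds a listener to its OnCommandIssued event.
; An Attack command launches the character upward and horizontally, using TargetMob's scaled world location as velocity rather than a direction toward it.
; No other command is handled, and nothing here sets TargetMob.
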(event `self.ReceiveBeginPlay`
  (bind _returnvalue (`GameplayStatics.GetActorOfClass` "/Game/Prototype/Blueprints/Rythm_manager_BP.Rythm_manager_BP_C"))
  (bind _output_get (set `self.RythmManagerRef` _returnvalue))
  (add `/Game/Prototype/Blueprints/Rythm_manager_BP.OnCommandIssued` _output_get (delegate `ListenToCommand`)))

(event `ListenToCommand`
  (params (Command :type "/Game/Prototype/Enums/E_CommandType Enum" :default "NewEnumerator0"))
  (switch `/Game/Prototype/Enums/E_CommandType` Command
    (:`NewEnumerator1`
      (`self.LaunchCharacter` (+ (* (`self.K2_GetActorLocation` (`self.TargetMob`)) 300.0) (0.0 0.0 300.0)) true true))))

(event `self.ReceiveTick`
  (params (DeltaSeconds :type "Float (single-precision)"))
  (if true
    _))

(fn `UserConstructionScript`)