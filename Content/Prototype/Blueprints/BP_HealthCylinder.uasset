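; BP_HealthCylinder is a cylinder actor that serves as a visual health indicator for the BP_Carriage_2 carriage.
; The construction script creates a dynamic instance of M_HealthCylinder on the mesh.
; On BeginPlay it finds the carriage by class and binds to its BPC_HealthComponent health-change event.
; Each change writes the new current health, without conversion, into the material's HealthPercentage parameter to alter the light emission.
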(event `self.ReceiveBeginPlay`
  (bind _returnvalue (`GameplayStatics.GetActorOfClass` "/Game/Prototype/Blueprints/BP_Carriage_2.BP_Carriage_2_C"))
  (bind _output_get (set `self.HealthComponentRef` (`self.GetComponentByClass` _returnvalue "/Game/Prototype/Blueprints/BPC_HealthComponent.BPC_HealthComponent_C")))
  (add `/Game/Prototype/Blueprints/BPC_HealthComponent.OnHealthChanged` _output_get (delegate `ChangeLightEmission`)))

(event `ChangeLightEmission`
  (params (NewCurrentHealth :type "Float (double-precision)"))
  (`MaterialInstanceDynamic.SetScalarParameterValue` (`self.DynamicMaterialRef`) "HealthPercentage" NewCurrentHealth))

(fn `UserConstructionScript`
  (bind _returnvalue (`PrimitiveComponent.CreateDynamicMaterialInstance` (`self.Cylinder`) 0 "/Game/Prototype/Materials/M_HealthCylinder.M_HealthCylinder" "None"))
  (set `self.DynamicMaterialRef` _returnvalue))