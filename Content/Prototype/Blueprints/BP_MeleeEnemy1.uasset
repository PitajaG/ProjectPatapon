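; Prototype melee enemy character that wakes when BP_Carriage enters its detection zone and acts on the rhythm manager's beat signal.
; Each beat it leaps toward the rhythm manager's location until the carriage reaches its hitbox.
; It then flashes brighter through a dynamic material over three beats, damaging overlapping carriages' health components on the third.
; The end-overlap reset is unconnected, so the in-range flag never clears.
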(event `self.ReceiveBeginPlay`
  ; Set Rythm Manager Reference
  (bind _returnvalue (`GameplayStatics.GetActorOfClass` "/Game/Prototype/Blueprints/Rythm_manager_BP.Rythm_manager_BP_C"))
  (set `self.RythmManagerRef` _returnvalue))

(event `self.DetectionZone.OnComponentBeginOverlap`
  (params (OverlappedComponent :type "PrimitiveComponent Object Reference") (OtherActor :type "Actor Object Reference") (OtherComp :type "PrimitiveComponent Object Reference") (OtherBodyIndex :type Integer) (bFromSweep :type Boolean) (SweepResult :type "HitResult Structure (by ref)"))
  ; If player in detection range, activate
  (bind _asbp_carriage (castclass `/Game/Prototype/Blueprints/BP_Carriage` (`GameplayStatics.GetObjectClass` OtherActor)))
  (if (== (`GameplayStatics.GetObjectClass` OtherActor) _asbp_carriage)
    (set `self.Carriage Ref` OtherActor)
    (bind _output_get (set `self.IsActive` true))
    ; Connecting event to Beat Signal
    (add `/Game/Prototype/Blueprints/Rythm_manager_BP.Beat Signal` (`self.RythmManagerRef`) (delegate `MoveOnBeat`))))

(event `MoveOnBeat`
  ; Connecting event to Beat Signal
  (if (stale `self.DetectionZone.OnComponentBeginOverlap` _output_get)
    (if (`self.PlayerInAttackRange`)
      ; Placeholder attack logic
      (`MovementComponent.StopMovementImmediately` (`self.CharacterMovement`))
      (bind _output_get (set `self.AttackCouter` (+ (`self.AttackCouter`) 1)))
      (switch `int` _output_get
        (:`1`
          ;; Increasing brightness each beat signal
          (bind _output_get_2 (set `self.FlashValue` 0.1))
          (`MaterialInstanceDynamic.SetScalarParameterValue` (`self.Dynamicmaterial`) "FlashValue" _output_get_2 :!label _label))
        (:`2`
          (set `self.FlashValue` 0.5)
          (goto _label))
        (:`3`
          (bind _output_get_3 (set `self.FlashValue` 10.0))
          (`MaterialInstanceDynamic.SetScalarParameterValue` (`self.Dynamicmaterial`) "FlashValue" _output_get_3)
          (`self.ApplyDamage`)
          (`MaterialInstanceDynamic.SetScalarParameterValue` (`self.Dynamicmaterial`) "FlashValue" 0.0)
          (set `self.AttackCouter` 0)))
      (else
        ; Jump towards the player on beat, until he's in attack range
        (if (`NavMovementInterface.IsMovingOnGround` (`self.CharacterMovement`))
          (`self.LaunchCharacter` (`KismetMathLibrary.MakeVector` (.x (* (`KismetMathLibrary.GetDirectionUnitVector` (`self.K2_GetActorLocation` self) (`self.K2_GetActorLocation` (`self.RythmManagerRef`))) 400.0)) (.y (* (`KismetMathLibrary.GetDirectionUnitVector` (`self.K2_GetActorLocation` self) (`self.K2_GetActorLocation` (`self.RythmManagerRef`))) 400.0)) 1000.0) true true))))))

(event `self.HitBox.OnComponentBeginOverlap`
  (params (OverlappedComponent :type "PrimitiveComponent Object Reference") (OtherActor :type "Actor Object Reference") (OtherComp :type "PrimitiveComponent Object Reference") (OtherBodyIndex :type Integer) (bFromSweep :type Boolean) (SweepResult :type "HitResult Structure (by ref)"))
  ; If player in Attack range, set flag
  (bind _asbp_carriage (castclass `/Game/Prototype/Blueprints/BP_Carriage` (`GameplayStatics.GetObjectClass` OtherActor)))
  (if (== (`GameplayStatics.GetObjectClass` OtherActor) _asbp_carriage)
    (set `self.PlayerInAttackRange` true)))

(event `self.HitBox.OnComponentEndOverlap`
  (params (OverlappedComponent :type "PrimitiveComponent Object Reference") (OtherActor :type "Actor Object Reference") (OtherComp :type "PrimitiveComponent Object Reference") (OtherBodyIndex :type Integer))
  ; If player not in Attack range anymore, reset flag
)

(fn `ApplyDamage`
  (for _array_element (`PrimitiveComponent.GetOverlappingActors` (`self.HitBox`) "/Game/Prototype/Blueprints/BP_Carriage.BP_Carriage_C")
    (`/Game/Prototype/Blueprints/BPC_HealthComponent.TakeDamage` (`self.GetComponentByClass` _array_element "/Game/Prototype/Blueprints/BPC_HealthComponent.BPC_HealthComponent_C") 25.0)))

(fn `UserConstructionScript`
  (bind _returnvalue (`PrimitiveComponent.CreateDynamicMaterialInstance` (`self.Mesh`) 1 "/Game/Prototype/Materials/M_MobIndicator.M_MobIndicator" "None"))
  (set `self.DynamicMaterial` _returnvalue))