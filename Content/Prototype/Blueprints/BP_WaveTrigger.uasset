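; BP_WaveTrigger is a trigger actor that spawns one wave of enemies when a BP_Carriage overlaps it.
; A DoOnce keeps the wave from repeating, then a loop spawns EnemiesToSpawn instances of EnemyClass.
; Enemies line up SpawnDistance ahead of the carriage, raised and offset along its right vector around the center, and turned to face back toward it.
; Despite a comment mentioning random locations, the placement is deterministic.
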(event `self.Wave Trigger.OnComponentBeginOverlap`
  (params (OverlappedComponent :type "PrimitiveComponent Object Reference") (OtherActor :type "Actor Object Reference") (OtherComp :type "PrimitiveComponent Object Reference") (OtherBodyIndex :type Integer) (bFromSweep :type Boolean) (SweepResult :type "HitResult Structure (by ref)"))
  (bind _wavecarriageref (`self.WaveCarriageRef`))
  (bind _asbp_carriage (cast `/Game/Prototype/Blueprints/BP_Carriage` OtherActor))
  (set `self.WaveCarriageRef` _asbp_carriage)
  ; So the wave doesnt trigger multiple times
  (`/Engine/EditorBlueprintResources/StandardMacros.DoOnce` false
    (:`Completed`
      (for _index (range 1 (+ (`self.EnemiesToSpawn`) 1))
        (`|SpawnActorFromClass` (`self.EnemyClass`) (`KismetMathLibrary.MakeTransform` (+ (+ (`self.K2_GetActorLocation` _wavecarriageref) (* (`self.GetActorForwardVector` _wavecarriageref) (`self.SpawnDistance`)) (0.0 0.0 0.0)) (* (`self.GetActorRightVector` _wavecarriageref) (* (- _index (/ (+ (`self.EnemiesToSpawn`) 1) 2)) 200.0)) (0.0 0.0 200.0)) (`KismetMathLibrary.ComposeRotators` (`self.K2_GetActorRotation` _wavecarriageref) (struct :`Pitch` 180.0))) "Undefined" "MultiplyWithRoot" null null)))))

(fn `UserConstructionScript`)