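; BPC_HealthComponent is a prototype health component that tracks current health, starting from its maximum at BeginPlay.
; It finds the Rythm_manager_BP actor in the level and binds to its OnCommandIssued event, where only the Recall command triggers a fixed amount of damage.
; TakeDamage subtracts from current health without clamping or a death check, then broadcasts the new value through OnHealthChanged.
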(event `self.ReceiveBeginPlay`
  (set `self.CurrentHealth` (`self.MaxHealth`))
  (bind _returnvalue (`GameplayStatics.GetActorOfClass` "/Game/Prototype/Blueprints/Rythm_manager_BP.Rythm_manager_BP_C"))
  (bind _output_get (set `self.RythmManagerRef` _returnvalue))
  (add `/Game/Prototype/Blueprints/Rythm_manager_BP.OnCommandIssued` _output_get (delegate `TakeDamageFromCommand`)))

(event `TakeDamageFromCommand`
  (params (Command :type "/Game/Prototype/Enums/E_CommandType Enum" :default "NewEnumerator0"))
  (switch `/Game/Prototype/Enums/E_CommandType` Command
    (:`NewEnumerator4`
      (`self.TakeDamage` 25.0))))

(event `TakeDamage`
  (params (Damage :type "Float (double-precision)"))
  (bind _output_get (set `self.CurrentHealth` (- (`self.CurrentHealth`) Damage)))
  (`self.OnHealthChanged` _output_get))