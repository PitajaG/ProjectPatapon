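; Rhythm manager actor that broadcasts music beats and turns drum-hit sequences into march, attack, defend or recall commands.
; Each FMOD timeline beat fires a beat signal and briefly flashes the cylinder's dynamic material.
; RegisterDrumHit buffers four hits, then ProcessCommand compares them to pattern arrays, dispatches any matching command and clears the buffer.
; CheckRythmAccuracy is an unfinished timing check: song position is fixed at zero and nothing here calls it.
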(event `self.ReceiveBeginPlay`
  ; BPM and dynamic material instance setting
  (set `self.BeatInterval` (/ 60.0 (`self.BPM`)))
  (bind _returnvalue (`PrimitiveComponent.CreateDynamicMaterialInstance` (`self.Cylinder`) 0 "/Game/Prototype/Materials/M_RythmManager.M_RythmManager" "None"))
  (set `self.DynamicMaterial` _returnvalue))

(event `self.FMODAudio.OnTimelineBeat`
  (params (Bar :type Integer) (Beat :type Integer) (Position :type Integer) (Tempo :type "Float (single-precision)") (TimeSignatureUpper :type Integer) (TimeSignatureLower :type Integer))
  (`self.Beat Signal`)
  (`MaterialInstanceDynamic.SetScalarParameterValue` (`self.DynamicMaterial`) "FlashStrength" 10.0)
  (`KismetSystemLibrary.Delay` 0.2)
  (`MaterialInstanceDynamic.SetScalarParameterValue` (`self.DynamicMaterial`) "FlashStrength" 0.0))

(fn `CheckRythmAccuracy`
  (returns (IsOnBeat :type Boolean))
  (locals (TimeInBeat :type "Float (double-precision)" :default 0.0))
  ; Current song position
  (set `local.TimeInBeat` (mod 0.0 (`self.BeatInterval`)))
  (return (or (< (`local.TimeInBeat`) (`self.InputTolerance`)) (> (`local.TimeInBeat`) (- (`self.BeatInterval`) (`self.InputTolerance`))))))

(fn `ProcessCommand`
  (`|ExecutionSequence`
    (:`then_0`
      ; March branch
      (if (`KismetArrayLibrary.Array_Identical` (`self.CurrentSequence`) (`self.Pattern_March`))
        (`self.OnCommandIssued` "NewEnumerator2")
        (`KismetArrayLibrary.Array_Clear` (`self.CurrentSequence`))
        (`KismetSystemLibrary.PrintString` "March command Sent")))
    (:`then_1`
      ; Attack branch
      (if (`KismetArrayLibrary.Array_Identical` (`self.CurrentSequence`) (`self.Pattern_Attack`))
        (`self.OnCommandIssued` "NewEnumerator1")
        (`KismetArrayLibrary.Array_Clear` (`self.CurrentSequence`))
        (`KismetSystemLibrary.PrintString` "Attack command Sent")))
    (:`then_2`
      ; Defend branch
      (if (`KismetArrayLibrary.Array_Identical` (`self.CurrentSequence`) (`self.Pattern_Defend`))
        (`self.OnCommandIssued` "NewEnumerator3")
        (`KismetArrayLibrary.Array_Clear` (`self.CurrentSequence`))
        (`KismetSystemLibrary.PrintString` "Defend command Sent")))
    (:`then_3`
      ; Recall branch
      (if (`KismetArrayLibrary.Array_Identical` (`self.CurrentSequence`) (`self.Pattern_Recall`))
        (`self.OnCommandIssued` "NewEnumerator4")
        (`KismetArrayLibrary.Array_Clear` (`self.CurrentSequence`))))))

(fn `RegisterDrumHit`
  (params (HitDrum :type "/Game/Prototype/Enums/E_DrumType Enum" :default "NewEnumerator0"))
  (`KismetArrayLibrary.Array_Add` (`self.CurrentSequence`) HitDrum)
  (if (== (`KismetArrayLibrary.Array_Length` (`self.CurrentSequence`)) 4)
    (`self.ProcessCommand`)
    (`KismetArrayLibrary.Array_Clear` (`self.CurrentSequence`))))

(fn `UserConstructionScript`)