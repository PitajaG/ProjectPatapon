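; BP_Drum_VR is a VR drum that reacts when struck by a grabbable drumstick, feeding hits into the rhythm game.
; A stick hit triggers stick vibration; if the impulse reaches a threshold, the drum plays its FMOD event and briefly flashes its dynamic material.
; It asks the rhythm manager to check timing and registers its drum type only on accurate hits.
; A short delayed DoOnce reset debounces repeated hits.
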(event `self.ReceiveBeginPlay`
  ; BeginPlay initialization
  ;; Initialazing dynamic materials
  (bind _returnvalue (`PrimitiveComponent.CreateDynamicMaterialInstance` (`self.DrumMesh`) 0 (`self.StaticMaterial`) "None"))
  (set `self.DynamicMaterial` _returnvalue)
  ;; Setting RythmManager reference
  (bind _returnvalue_2 (`GameplayStatics.GetActorOfClass` "/Game/Prototype/Blueprints/Rythm_manager_BP.Rythm_manager_BP_C"))
  (set `self.RythmManagerRef` _returnvalue_2))

(event `self.ReceiveHit`
  (params (MyComp :type "PrimitiveComponent Object Reference") (Other :type "Actor Object Reference") (OtherComp :type "PrimitiveComponent Object Reference") (bSelfMoved :type Boolean) (HitLocation :type "Vector Structure") (HitNormal :type "Vector Structure") (NormalImpulse :type "Vector Structure") (Hit :type "HitResult Structure (by ref)"))
  ; Hit event logic
  ;; If object that has hit the drum is of correct class, continue
  (bind _asgrabbable_drumsticks (castclass `/Game/Prototype/Blueprints/Drums/Grabbable_drumsticks` (`GameplayStatics.GetObjectClass` Other)))
  (bind _asgrabbable_drumsticks_2 (cast `/Game/Prototype/Blueprints/Drums/Grabbable_drumsticks` Other))
  (`/Game/Prototype/Blueprints/Drums/Grabbable_drumsticks.HitVibrate` _asgrabbable_drumsticks_2)
  (if (and (== (`GameplayStatics.GetObjectClass` Other) _asgrabbable_drumsticks) (>= (`KismetMathLibrary.VSize` NormalImpulse) (`self.HitThreshold`)))
    (`/Engine/EditorBlueprintResources/StandardMacros.DoOnce` false :!label _label
      (:`Completed`
        (`|ExecutionSequence`
          (:`then_0`
            ;; Playing FMod event and location of the drum
            (`FMODBlueprintStatics.PlayEventAtLocation` (`self.DrumFmodEvent`) (`KismetMathLibrary.Conv_VectorToTransform` (`self.K2_GetActorLocation`)))
            (`MaterialInstanceDynamic.SetScalarParameterValue` (`self.DynamicMaterial`) "FlashStrength" 10.0)
            (`KismetSystemLibrary.Delay` 0.2)
            (`MaterialInstanceDynamic.SetScalarParameterValue` (`self.DynamicMaterial`) "FlashStrength" 0.0))
          (:`then_1`
            ;; Checking rythm accuracy that detetrmines whether hit gets registered or not
            (bind _isonbeat (`/Game/Prototype/Blueprints/Rythm_manager_BP.CheckRythmAccuracy` (`self.RythmManagerRef`)))
            (if _isonbeat
              (`/Game/Prototype/Blueprints/Rythm_manager_BP.RegisterDrumHit` (`self.RythmManagerRef`) (`self.MyDrumType`))))
          (:`then_2`
            (`KismetSystemLibrary.Delay` 0.1)
            (goto _label :!via `Reset`)))))))

(fn `UserConstructionScript`)