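; BP_Knight is a prototype escort character that holds a formation offset beside BP_Carriage and acts on rhythm commands.
; Tick steers it toward the offset with movement input, using a small dead zone against twitching, and copies the carriage's yaw.
; Rythm_manager_BP commands trigger montages: Defend blocks, while Attack also destroys, after a short delay, "Enemy"-tagged actors tracked by DetectionZone overlaps.
; An unconnected Timeline-driven spline step movement remains unused.
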(event `self.ReceiveBeginPlay`
  (bind _returnvalue (`GameplayStatics.GetActorOfClass` "/Game/Prototype/Blueprints/BP_Carriage.BP_Carriage_C"))
  (set `self.CarriageRef` _returnvalue)
  (bind _returnvalue_2 (`GameplayStatics.GetActorOfClass` "/Game/Prototype/Blueprints/Rythm_manager_BP.Rythm_manager_BP_C"))
  (bind _output_get (set `self.RythmManagerRef` _returnvalue_2))
  (add `/Game/Prototype/Blueprints/Rythm_manager_BP.OnCommandIssued` _output_get (delegate `ListenToCommand`)))

(event `ListenToCommand`
  (params (Command :type "/Game/Prototype/Enums/E_CommandType Enum" :default "NewEnumerator0"))
  (switch `/Game/Prototype/Enums/E_CommandType` Command
    (:`NewEnumerator1`
      ; Attack logic
      (`self.PlayAnimMontage` "/Game/Prototype/Meshes/Knight_Attack.Knight_Attack")
      (`KismetSystemLibrary.Delay` 0.1)
      (for _array_element (`self.EnemiesInZone`)
        (`self.K2_DestroyActor` _array_element)))
    (:`NewEnumerator3`
      ; Defend Anim
      (`self.PlayAnimMontage` "/Game/Prototype/Meshes/Knight_Block.Knight_Block"))))

(event `self.DetectionZone.OnComponentBeginOverlap`
  (params (OverlappedComponent :type "PrimitiveComponent Object Reference") (OtherActor :type "Actor Object Reference") (OtherComp :type "PrimitiveComponent Object Reference") (OtherBodyIndex :type Integer) (bFromSweep :type Boolean) (SweepResult :type "HitResult Structure (by ref)"))
  ; Add Enemy to Array
  (if (`self.ActorHasTag` OtherActor "Enemy")
    (`KismetArrayLibrary.Array_AddUnique` (`self.EnemiesInZone`) OtherActor)))

(event `self.DetectionZone.OnComponentEndOverlap`
  (params (OverlappedComponent :type "PrimitiveComponent Object Reference") (OtherActor :type "Actor Object Reference") (OtherComp :type "PrimitiveComponent Object Reference") (OtherBodyIndex :type Integer))
  ; Remove Enemy From Array
  (if (`self.ActorHasTag` OtherActor "Enemy")
    (`KismetArrayLibrary.Array_RemoveItem` (`self.EnemiesInZone`) OtherActor)))

(event `self.ReceiveTick`
  (params (DeltaSeconds :type "Float (single-precision)"))
  (bind _carriageref (`self.CarriageRef`))
  (bind _returnvalue (- (`KismetMathLibrary.TransformLocation` (`self.GetTransform` _carriageref) (`self.FormationOffset`)) (`self.K2_GetActorLocation`)))
  ; Knight movement
  (`|ExecutionSequence`
    (:`then_0`
      (if (> (`KismetMathLibrary.VSize` _returnvalue) 10.0)
        (`self.AddMovementInput` (`KismetMathLibrary.Normal` _returnvalue))))
    (:`then_1`
      (`self.K2_SetActorRotation` (`KismetMathLibrary.MakeRotator` 0.0 0.0 (.yaw (`self.K2_GetActorRotation` _carriageref)))))))

(fn `UserConstructionScript`)