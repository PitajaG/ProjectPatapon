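; BP_Guardian is a prototype guardian actor that responds to commands from the rhythm manager by clearing nearby enemies.
; On BeginPlay it finds Rythm_manager_BP and binds a listener to its OnCommandIssued event.
; DetectionZone overlap events keep EnemiesInZone filled with actors tagged "Enemy".
; The Attack command, the only one handled, destroys every actor in that array, with no single-target selection or damage step.
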(event `self.ReceiveBeginPlay`
  (bind _returnvalue (`GameplayStatics.GetActorOfClass` "/Game/Prototype/Blueprints/Rythm_manager_BP.Rythm_manager_BP_C"))
  (bind _output_get (set `self.RythmManagerRef` _returnvalue))
  (add `/Game/Prototype/Blueprints/Rythm_manager_BP.OnCommandIssued` _output_get (delegate `ListenToCommand`)))

(event `ListenToCommand`
  (params (Command :type "/Game/Prototype/Enums/E_CommandType Enum" :default "NewEnumerator0"))
  (switch `/Game/Prototype/Enums/E_CommandType` Command
    (:`NewEnumerator1`
      ; Attack logic
      ;; Get Current Target
      (for _array_element (`self.EnemiesInZone`)
        (`self.K2_DestroyActor` _array_element)))))

(event `self.DetectionZone.OnComponentBeginOverlap`
  (params (OverlappedComponent :type "PrimitiveComponent Object Reference") (OtherActor :type "Actor Object Reference") (OtherComp :type "PrimitiveComponent Object Reference") (OtherBodyIndex :type Integer) (bFromSweep :type Boolean) (SweepResult :type "HitResult Structure (by ref)"))
  ; Add Enemy to Array
  (if (`self.ActorHasTag` OtherActor "Enemy")
    (`KismetArrayLibrary.Array_Add` (`self.EnemiesInZone`) OtherActor)))

(event `self.DetectionZone.OnComponentEndOverlap`
  (params (OverlappedComponent :type "PrimitiveComponent Object Reference") (OtherActor :type "Actor Object Reference") (OtherComp :type "PrimitiveComponent Object Reference") (OtherBodyIndex :type Integer))
  ; Remove Enemy From Array
  (if (`self.ActorHasTag` OtherActor "Enemy")
    (`KismetArrayLibrary.Array_RemoveItem` (`self.EnemiesInZone`) OtherActor)))

(fn `UserConstructionScript`)