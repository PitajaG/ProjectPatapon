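; Actor component for BP_Carriage that offers three distinct random upgrades and applies the chosen healing, max health or move speed boost.
; Each pick rolls a rarity against cumulative thresholds, then draws randomly from matching DT_Upgrade rows, re-rolling when none remain.
; The selection pauses the game and shows WBP_UpgradeSelection, either on an actor spawned facing the VR camera or in the desktop viewport.
; Applying an upgrade closes the menu and unpauses.
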(event `self.ReceiveBeginPlay`
  (bind _asbp_carriage (cast `/Game/Prototype/Blueprints/Player/BP_Carriage` (`self.GetOwner`)))
  (set `self.Owner` _asbp_carriage))

(event `DisplayUpgradeSelection`
  (`self.RollNewUpgrades`)
  (`self.ShowUI`))

(event `ApplyUpgrade`
  (params (Upgrade :type "/Game/Prototype/DataTable/ST_Upgrade Structure"))
  (`self.SwitchUpgrade` Upgrade)
  (`self.HideUI`))

(fn `HideUI`
  (bind _returnvalue (`GameplayStatics.GetPlayerController` 0))
  (if (`self.bIsVRLevel`)
    ; VR
    (`Actor.K2_DestroyActor` (`self.CurrentVRUpgradeMenu`))
    (`GameplayStatics.SetGamePaused` false)
    (bind _asvrplayer (cast `/Game/Prototype/Blueprints/Player/VRPlayer` (`GameplayStatics.GetPlayerPawn` 0)))
    (set `WidgetInteractionComponent.bShowDebug` false (`/Game/Prototype/Blueprints/Player/VRPlayer.WidgetInteractionRight` _asvrplayer))
    (else
      ; Desktop
      (`WidgetBlueprintLibrary.SetInputMode_GameOnly` _returnvalue)
      (set `PlayerController.bShowMouseCursor` false _returnvalue)
      (`Widget.RemoveFromParent` (`self.UpgradeWidget`))
      (`GameplayStatics.SetGamePaused` false))))

(fn `RollNewUpgrades`
  (locals (MatchingUpgrades :type "Array of /Game/Prototype/DataTable/ST_Upgrade Structure"))
  (bind _matchingupgrades (`local.MatchingUpgrades`))
  (`KismetArrayLibrary.Array_Clear` (`self.SelectedUpgrades`))
  (for _ (range 3)
    (`KismetArrayLibrary.Array_Clear` (`local.MatchingUpgrades`) :!label _label)
    (bind _newparam (`self.RollRarity`))
    (bind _outrownames (`DataTableFunctionLibrary.GetDataTableRowNames` "/Game/Prototype/DataTable/DT_Upgrade.DT_Upgrade"))
    (for _array_element _outrownames
      (bind _returnvalue (`|GetDataTableRow` "/Game/Prototype/DataTable/DT_Upgrade.DT_Upgrade" _array_element)
        (:`then`
          (if (`|EnumEquality` (`.Rarity_19_56C95BF244DF5C03088511A526B9CF2E` (break `/Game/Prototype/DataTable/ST_Upgrade` _returnvalue)) _newparam)
            (if (not (`KismetArrayLibrary.Array_Contains` (`self.SelectedUpgrades`) _returnvalue))
              (`KismetArrayLibrary.Array_Add` (`local.MatchingUpgrades`) _returnvalue))))))
    (if (== (`KismetArrayLibrary.Array_Length` _matchingupgrades) 0)
      (goto _label)
      (else
        (`KismetArrayLibrary.Array_Add` (`self.SelectedUpgrades`) (`|GetArrayItem` _matchingupgrades (`KismetMathLibrary.RandomIntegerInRange` 0 (- (`KismetArrayLibrary.Array_Length` (`local.MatchingUpgrades`)) 1))))))))

(fn `RollRarity`
  (returns (NewParam :type "/Game/Prototype/Enums/E_Rarity Enum"))
  (locals (RandomFloat :type "Float (double-precision)") (OutRarity :type "/Game/Prototype/Enums/E_Rarity Enum") (Common :type "Float (double-precision)" :default 60.0) (Uncommon :type "Float (double-precision)" :default 85.0) (Rare :type "Float (double-precision)" :default 95.0) (Epic :type "Float (double-precision)" :default 99.0) (Legendary :type "Float (double-precision)" :default 100.0))
  (set `local.RandomFloat` (`KismetMathLibrary.RandomFloatInRange` 1.0 100.0))
  (if (<= (`local.RandomFloat`) (`local.Common`))
    (set `local.OutRarity` "NewEnumerator0")
    (elif (<= (`local.RandomFloat`) (`local.Uncommon`))
      (set `local.OutRarity` "NewEnumerator1")
      (elif (<= (`local.RandomFloat`) (`local.Rare`))
        (set `local.OutRarity` "NewEnumerator2")
        (elif (<= (`local.RandomFloat`) (`local.Epic`))
          (set `local.OutRarity` "NewEnumerator3")
          (else
            (set `local.OutRarity` "NewEnumerator4"))))))
  (`KismetSystemLibrary.PrintString` (`KismetStringLibrary.Conv_DoubleToString` (`local.RandomFloat`)) false false)
  (return (`local.OutRarity`)))

(fn `ShowUI`
  (bind _returnvalue (`GameplayStatics.GetPlayerCameraManager` 0))
  (bind _returnvalue_2 (`GameplayStatics.GetPlayerController` 0))
  (bind _returnvalue_3 (`PlayerCameraManager.GetCameraLocation` _returnvalue))
  (bind (_returnvalue_x _returnvalue_y) (`KismetMathLibrary.BreakVector` (+ (* (`KismetMathLibrary.Normal` (`KismetMathLibrary.MakeVector` (.x (`KismetMathLibrary.GetForwardVector` (`PlayerCameraManager.GetCameraRotation` (`GameplayStatics.GetPlayerCameraManager` 0)))) (.y (`KismetMathLibrary.GetForwardVector` (`PlayerCameraManager.GetCameraRotation` (`GameplayStatics.GetPlayerCameraManager` 0)))))) (350.0 350.0 350.0)) _returnvalue_3)))
  (if (`self.bIsVRLevel`)
    ; VR
    (bind _returnvalue_4 (`|SpawnActorFromClass` "/Game/Prototype/UI/BP_UpgradeSelectionVR.BP_UpgradeSelectionVR_C" (`KismetMathLibrary.MakeTransform` (`KismetMathLibrary.MakeVector` _returnvalue_x _returnvalue_y (.z _returnvalue_3)) (`KismetMathLibrary.MakeRotator` 0.0 0.0 (+ (.yaw (`PlayerCameraManager.GetCameraRotation` _returnvalue)) 180.0))) "Undefined" "MultiplyWithRoot" null null))
    (set `self.CurrentVRUpgradeMenu` _returnvalue_4)
    (bind _aswbp_upgrade_selection (cast `/Game/Prototype/UI/WBP_UpgradeSelection` (`WidgetComponent.GetWidget` (`/Game/Prototype/UI/BP_UpgradeSelectionVR.Widget` (`self.CurrentVRUpgradeMenu`)))))
    (set `/Game/Prototype/UI/WBP_UpgradeSelection.UpgradeComponent` self _aswbp_upgrade_selection)
    (`/Game/Prototype/UI/WBP_UpgradeSelection.InitSelection` _aswbp_upgrade_selection (`self.SelectedUpgrades`))
    (`GameplayStatics.SetGamePaused` true)
    (bind _asvrplayer (cast `/Game/Prototype/Blueprints/Player/VRPlayer` (`GameplayStatics.GetPlayerPawn` 0)))
    (set `WidgetInteractionComponent.bShowDebug` true (`/Game/Prototype/Blueprints/Player/VRPlayer.WidgetInteractionRight` _asvrplayer))
    (else
      ; Desktop
      (bind _returnvalue_5 (`|CreateWidget` "/Game/Prototype/UI/WBP_UpgradeSelection.WBP_UpgradeSelection_C" (`GameplayStatics.GetPlayerController` 0)))
      (set `self.UpgradeWidget` _returnvalue_5)
      (set `/Game/Prototype/UI/WBP_UpgradeSelection.UpgradeComponent` self _returnvalue_5)
      (`/Game/Prototype/UI/WBP_UpgradeSelection.InitSelection` _returnvalue_5 (`self.SelectedUpgrades`))
      (`UserWidget.AddToViewport` _returnvalue_5 0)
      (`WidgetBlueprintLibrary.SetInputMode_UIOnlyEx` _returnvalue_2 null)
      (set `PlayerController.bShowMouseCursor` true _returnvalue_2)
      (`GameplayStatics.SetGamePaused` true))))

(fn `SwitchUpgrade`
  (params (Upgrade :type "/Game/Prototype/DataTable/ST_Upgrade Structure"))
  (bind _owner (`self.Owner`))
  (bind _bpc_healthcomponent (`/Game/Prototype/Blueprints/Player/BP_Carriage.BPC_HealthComponent` (`self.Owner`)))
  (switch `/Game/Prototype/Enums/E_UpgradeType` Upgrade_Type_17_F174575E483A4F9F6B92A29EB44D9244
    (:`NewEnumerator0`
      ;[0 1 0.08372 0.1] Healing
      (`/Game/Prototype/Blueprints/BPC/BPC_HealthComponent.AddHealth` (`/Game/Prototype/Blueprints/Player/BP_Carriage.BPC_HealthComponent` (`self.Owner`)) Upgrade_Value_18_E3638ED9451F1A2165A33E8F66FE0609))
    (:`NewEnumerator1`
      ;[1 0 0 0.1] Max Health Up
      (set `/Game/Prototype/Blueprints/BPC/BPC_HealthComponent.MaxHealth` (+ (`/Game/Prototype/Blueprints/BPC/BPC_HealthComponent.MaxHealth` _bpc_healthcomponent) Upgrade_Value_18_E3638ED9451F1A2165A33E8F66FE0609) _bpc_healthcomponent))
    (:`NewEnumerator2`
      ;[0.000115 0.9703 1 0.1] Speed Up
      (set `/Game/Prototype/Blueprints/Player/BP_Carriage.MoveSpeed` (+ (`/Game/Prototype/Blueprints/Player/BP_Carriage.MoveSpeed` _owner) Upgrade_Value_18_E3638ED9451F1A2165A33E8F66FE0609) _owner))))