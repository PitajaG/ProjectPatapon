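; BPC_HealthComponent is an actor component that tracks its owner's health.
; It fills health to the maximum at BeginPlay and caches a Rythm_manager_BP reference that this graph never uses.
; AddHealth caps healing at the maximum, while TakeDamage subtracts without clamping, and both broadcast OnHealthChanged.
; When damage brings health to zero or below, it sends OnDeathMessage to the owner, which handles the death.
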(event `self.ReceiveBeginPlay`
  ; Setting max current health and rythm manager ref
  (set `self.CurrentHealth` (`self.MaxHealth`))
  (bind _returnvalue (`GameplayStatics.GetActorOfClass` "/Game/Prototype/Blueprints/Rythm_manager_BP.Rythm_manager_BP_C"))
  (set `self.RythmManagerRef` _returnvalue))

(event `AddHealth`
  (params (Health :type "Float (double-precision)"))
  ; Add health
  (bind _output_get (set `self.CurrentHealth` (`KismetMathLibrary.FMin` (+ (`self.CurrentHealth`) Health) (`self.MaxHealth`))))
  (`self.OnHealthChanged` _output_get))

(event `TakeDamage`
  (params (Damage :type "Float (double-precision)"))
  ; Taking damage
  (bind _output_get (set `self.CurrentHealth` (- (`self.CurrentHealth`) Damage)))
  (`self.OnHealthChanged` _output_get)
  (if (<= (`self.CurrentHealth`) 0.0)
    (message `/Game/Prototype/Interfaces/BPI_Killable.OnDeath` (`self.GetOwner`))))