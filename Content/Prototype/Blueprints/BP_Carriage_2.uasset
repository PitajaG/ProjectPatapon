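; Carriage actor that carries drums and advances along a spline when the rhythm manager issues a March command.
; On BeginPlay it attaches each listed drum to itself and, within that same loop, binds to the manager's OnCommandIssued.
; Each March plays a timeline that lerps spline distance by one step length.
; A downward trace keeps it at a fixed height above the ground while rotation follows the spline.
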(event `self.ReceiveBeginPlay`
  ; Attach drums to carriage
  (for _array_element (`self.AttachedDrums`)
    (`self.K2_AttachToActor` _array_element self "None" "KeepWorld" "KeepWorld" "KeepWorld" true)
    ; Set rythm manager reference and bind event to OnCommandIssued function
    (bind _returnvalue (`GameplayStatics.GetActorOfClass` "/Game/Prototype/Blueprints/Rythm_manager_BP.Rythm_manager_BP_C"))
    (bind _output_get (set `self.RythmManagerRef` _returnvalue))
    (add `/Game/Prototype/Blueprints/Rythm_manager_BP.OnCommandIssued` _output_get (delegate `ListenToCommand`))))

(event `ListenToCommand`
  (params (Command :type "/Game/Prototype/Enums/E_CommandType Enum" :default "NewEnumerator0"))
  (bind _spline (`/Game/Prototype/Blueprints/BP_Path.Spline` (`self.SplineRef`)))
  ; Set rythm manager reference and bind event to OnCommandIssued function
  (switch `/Game/Prototype/Enums/E_CommandType` Command
    (:`NewEnumerator2`
      (set `self.CurrentDistance` (`self.LiveDistance`))
      (set `self.TargetDistance` (+ (`self.CurrentDistance`) (`self.StepLength`)))
      (bind (_direction _newtrack_0) (`Timeline|MarchTimeline` :!via `PlayFromStart`)
        (:`Update`
          (bind _output_get (set `self.LiveDistance` (`KismetMathLibrary.Lerp` (`self.CurrentDistance`) (`self.TargetDistance`) _newtrack_0)))
          (bind _output_get_2 (set `self.SplinePos` (`SplineComponent.GetLocationAtDistanceAlongSpline` _spline _output_get "World")))
          (bind (_outhit _returnvalue) (`KismetSystemLibrary.LineTraceSingle` _output_get_2 (- _output_get_2 (0.0 0.0 10000.0)) "TraceTypeQuery1"))
          (if _returnvalue
            (`self.K2_SetActorLocationAndRotation` (+ (`.ImpactPoint` (`GameplayStatics.BreakHitResult` _outhit)) (0.0 0.0 100.0)) (`SplineComponent.GetRotationAtDistanceAlongSpline` _spline _output_get "World"))))))))

(fn `UserConstructionScript`)