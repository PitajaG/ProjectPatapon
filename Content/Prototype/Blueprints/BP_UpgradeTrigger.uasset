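; BP_UpgradeTrigger is a one-use pickup that grants a random upgrade to the BP_Carriage.
; Any overlap on its Collision component, with no check on the overlapping actor, fetches the carriage via GetActorOfClass.
; A random switch adds health or max health through BPCHealthComponent, or raises MoveSpeed, then destroys the trigger.
; The fourth, debug-print branch is unreachable, as RandomInteger(3) yields only three outcomes.
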(event `self.Collision.OnComponentBeginOverlap`
  (params (OverlappedComponent :type "PrimitiveComponent Object Reference") (OtherActor :type "Actor Object Reference") (OtherComp :type "PrimitiveComponent Object Reference") (OtherBodyIndex :type Integer) (bFromSweep :type Boolean) (SweepResult :type "HitResult Structure (by ref)"))
  (bind _returnvalue (`GameplayStatics.GetActorOfClass` "/Game/Prototype/Blueprints/BP_Carriage.BP_Carriage_C"))
  (switch `int` (`KismetMathLibrary.RandomInteger` 3)
    (:`0`
      (bind _bpc_healthcomponent (`/Game/Prototype/Blueprints/BP_Carriage.BPC_HealthComponent` _returnvalue))
      ;[0 1 0.08372 0.1] Add Current Health
      (`/Game/Prototype/Blueprints/BPC_HealthComponent.AddHealth` _bpc_healthcomponent 50.0)
      (`self.K2_DestroyActor` :!label _label))
    (:`1`
      ;[1 0 0 0.1] Add Max Health
      (set `/Game/Prototype/Blueprints/BPC_HealthComponent.MaxHealth` (+ (`/Game/Prototype/Blueprints/BPC_HealthComponent.MaxHealth` _bpc_healthcomponent) 25.0) _bpc_healthcomponent)
      (goto _label))
    (:`2`
      ;[0.000115 0.9703 1 0.1] Add max speed
      (set `/Game/Prototype/Blueprints/BP_Carriage.MoveSpeed` (+ (`/Game/Prototype/Blueprints/BP_Carriage.MoveSpeed` _returnvalue) 0.25) _returnvalue)
      (goto _label))
    (:`3`
      (`KismetSystemLibrary.PrintString` "Something not right"))))

(fn `UserConstructionScript`)