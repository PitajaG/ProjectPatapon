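; BP_Boss is a rhythm-driven boss that lobs boulders on a looping timer until the carriage enters its fight range.
; In the arena it counts Rythm_manager_BP beat signals, with a placeholder warning print before each periodic attack.
; Each attack randomly spawns two ranged enemies, a melee enemy or a deflectable boulder.
; Deflectable projectiles overlapping its capsule damage its health component, and OnDeath destroys the actor.
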(event `ThrowBoulderTimer`
  ; Throwing boulder without bossfight
  (if (not (`self.IsInArena`))
    (`|SpawnActorFromClass` "/Game/Prototype/Blueprints/BP_Boulder.BP_Boulder_C" (`SceneComponent.K2_GetComponentToWorld` (`self.BoulderSpawn`)) "AdjustIfPossibleButAlwaysSpawn" "MultiplyWithRoot" null (`SceneComponent.K2_GetComponentLocation` (`self.BoulderSpawn`)) 5.0 120.0 false null)))

(event `self.ReceiveBeginPlay`
  ; Setting references
  (`KismetSystemLibrary.K2_SetTimerDelegate` (delegate `ThrowBoulderTimer`) 20.0 true)
  (bind _returnvalue (`GameplayStatics.GetActorOfClass` "/Game/Prototype/Blueprints/Rythm_manager_BP.Rythm_manager_BP_C"))
  (set `self.RythmManagerRef` _returnvalue)
  (bind _returnvalue_2 (`GameplayStatics.GetActorOfClass` "/Game/Prototype/Blueprints/BP_Carriage.BP_Carriage_C"))
  (set `self.CarriageRef` _returnvalue_2)
  ; Connecting boss logic to beat signal
  (add `/Game/Prototype/Blueprints/Rythm_manager_BP.Beat Signal` (`self.RythmManagerRef`) (delegate `BeatSignal`)))

(event `BeatSignal`
  ; Connecting boss logic to beat signal
  ; BeatCounter
  (if (`self.IsInArena`)
    (`|ExecutionSequence`
      (:`then_0`
        (set `self.BeatCounter` (+ (`self.BeatCounter`) 1)))
      (:`then_1`
        (if (== (`self.BeatCounter`) 8)
          ; Incoming attack indicator
          (`KismetSystemLibrary.PrintString` "Hello")
          (else
            ; Calling attack sequence
            (if (== (`self.BeatCounter`) 10)
              (`self.AttackSequence`)
              (set `self.Attacking` true)
              (set `self.BeatCounter` 0))))))))

(event `AttackSequence`
  ; Attack loop logic
  (bind _output_get (set `self.AttackNumber` (`KismetMathLibrary.RandomIntegerInRange` 0 2)))
  (switch `int` _output_get
    (:`0`
      ;; Spawning ranged oponents
      (`|SpawnActorFromClass` "/Game/Prototype/Blueprints/BP_RangedEnemy.BP_RangedEnemy_C" (`self.GetTransform` (`self.LeftRangeSpawnPoint`)) "AdjustIfPossibleButAlwaysSpawn" "MultiplyWithRoot" null null)
      (`|SpawnActorFromClass` "/Game/Prototype/Blueprints/BP_RangedEnemy.BP_RangedEnemy_C" (`self.GetTransform` (`self.RightRangeSpawnPoint`)) "AdjustIfPossibleButAlwaysSpawn" "MultiplyWithRoot" null null))
    (:`1`
      ;; Spawning melee oponents
      (`|SpawnActorFromClass` "/Game/Prototype/Blueprints/BP_MeleeEnemy1.BP_MeleeEnemy1_C" (`self.GetTransform` (`self.MeleeSpawnPoint`)) "AdjustIfPossibleButAlwaysSpawn" "MultiplyWithRoot" null null))
    (:`2`
      ;; Throwing boulder
      (`|SpawnActorFromClass` "/Game/Prototype/Blueprints/BP_Boulder.BP_Boulder_C" (`SceneComponent.K2_GetComponentToWorld` (`self.BoulderSpawn`)) "AdjustIfPossibleButAlwaysSpawn" "MultiplyWithRoot" null (`SceneComponent.K2_GetComponentLocation` (`self.BoulderSpawn`)) 5.0 120.0 true null))))

(event `self.CapsuleComponent.OnComponentBeginOverlap`
  (params (OverlappedComponent :type "PrimitiveComponent Object Reference") (OtherActor :type "Actor Object Reference") (OtherComp :type "PrimitiveComponent Object Reference") (OtherBodyIndex :type Integer) (bFromSweep :type Boolean) (SweepResult :type "HitResult Structure (by ref)"))
  ; Damage from boulder
  (if (`KismetSystemLibrary.DoesImplementInterface` OtherActor "/Game/Prototype/Interfaces/BPI_DeflectableProjectile.BPI_DeflectableProjectile_C")
    (message `/Game/Prototype/Interfaces/BPI_DeflectableProjectile.OnProjectileHit` OtherActor)
    (`/Game/Prototype/Blueprints/BPC_HealthComponent.TakeDamage` (`self.BPC_HealthComponent`) 500.0)))

(event `/Game/Prototype/Interfaces/BPI_Killable.OnDeath`
  ; Death
  (`self.K2_DestroyActor`))

(event `self.BossFightRange.OnComponentBeginOverlap`
  (params (OverlappedComponent :type "PrimitiveComponent Object Reference") (OtherActor :type "Actor Object Reference") (OtherComp :type "PrimitiveComponent Object Reference") (OtherBodyIndex :type Integer) (bFromSweep :type Boolean) (SweepResult :type "HitResult Structure (by ref)"))
  ; Comment
  (if (== OtherActor (`self.CarriageRef`))
    (set `self.IsInArena` true)))

(fn `UserConstructionScript`)