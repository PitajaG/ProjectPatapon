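; Bomb projectile that flies in an arc toward BP_Carriage and can be deflected back at its thrower.
; Flight time snaps to whole beats at a hardcoded 120 BPM, setting the timeline play rate; arc height scales with distance.
; Timeline-driven lerps track the carriage's, or after deflection the thrower's, current position.
; On hit it hides, disables collision, spawns destruction particles and destroys itself after a delay.
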(event `self.ReceiveBeginPlay`
  ; Setting Carriage Ref
  (bind _returnvalue (`GameplayStatics.GetActorOfClass` "/Game/Prototype/Blueprints/BP_Carriage.BP_Carriage_C"))
  (set `self.CarriageRef` _returnvalue)
  ; Setting RythmManager Ref
  (bind _returnvalue_2 (`GameplayStatics.GetActorOfClass` "/Game/Prototype/Blueprints/Rythm_manager_BP.Rythm_manager_BP_C"))
  (set `self.RythmManagerRef` _returnvalue_2)
  ; Flight Adaptive to BPM
  (bind _boulderflighttime (`self.CalculateFlightTime` 120.0))
  (`self.CalculateFlightHight`)
  ; Adaptive playrate
  (`TimelineComponent.SetPlayRate` (`self.FlightTimeline`) (/ 1.0 _boulderflighttime))
  ; Setting starting location
  (set `self.StartLocation` (`self.K2_GetActorLocation` self))
  ; Flight based on timeline lerp with preset arch
  (bind (_direction _alpha _arch) (`Timeline|FlightTimeline` :!label _label)
    (:`Update`
      (`self.K2_SetActorLocation` (+ (`KismetMathLibrary.MakeVector` 0.0 0.0 (* _arch (`self.FlightHight`))) (`KismetMathLibrary.VLerp` (`self.StartLocation`) (`self.K2_GetActorLocation` (`self.CarriageRef`)) _alpha))))))

(event `self.OnProjectileDeflect`
  (bind _throwerref (`self.ThrowerRef`))
  ; Deflect logic
  (`/Engine/EditorBlueprintResources/StandardMacros.IsValid` (`self.ThrowerRef`)
    (:`Is Valid`
      (`|ExecutionSequence`
        (:`then_0`
          (goto _label :!via `Stop`))
        (:`then_1`
          (set `self.StartLocation` (`self.K2_GetActorLocation` self))
          (bind (_direction _alpha) (`Timeline|DeflectTimeline` :!via `PlayFromStart`)
            (:`Update`
              (`/Engine/EditorBlueprintResources/StandardMacros.IsValid` _throwerref
                (:`Is Valid`
                  (`self.K2_SetActorLocation` (`KismetMathLibrary.VLerp` (`self.StartLocation`) (`self.K2_GetActorLocation` _throwerref) _alpha))
                  (set `self.IsDeflected` true))))))))))

(event `self.OnProjectileHit`
  ; Projectile vfx and destruction
  (`|ExecutionSequence`
    (:`then_0`
      (goto _label :!via `Stop`))
    (:`then_1`
      (`self.SetActorHiddenInGame` true)
      (`PrimitiveComponent.SetCollisionEnabled` (`self.Sphere`) "NoCollision")
      (`PrimitiveComponent.SetCollisionEnabled` (`self.Sphere1`) "NoCollision")
      (`NiagaraFunctionLibrary.SpawnSystemAtLocation` "/Game/Prototype/Niagara/BoulderDestructionParticles.BoulderDestructionParticles" (`self.K2_GetActorLocation` self) (struct) (10.0 10.0 10.0))
      (`KismetSystemLibrary.Delay` 1.5)
      (`self.K2_DestroyActor`))))

(fn `CalculateFlightHight`
  (set `self.FlightHight` (`KismetMathLibrary.FClamp` (* (`self.DistanceToTarget`) 0.25) 300.0 1000000.0)))

(fn `CalculateFlightTime`
  (params (BPM :type "Float (double-precision)"))
  (returns (BoulderFlightTIme :type "Float (double-precision)"))
  (locals (AproxTime :type "Float (double-precision)") (BeatTime :type "Float (double-precision)"))
  (set `local.BeatTime` (/ 60.0 BPM))
  (bind _output_get (set `self.DistanceToTarget` (`KismetMathLibrary.VSizeXY` (- (`self.K2_GetActorLocation` (`self.CarriageRef`)) (`self.K2_GetActorLocation`)))))
  (bind _output_get_2 (set `local.AproxTime` (/ _output_get (`self.BaseSpeed`))))
  (return (* (`KismetMathLibrary.Max` (`KismetMathLibrary.Round` (/ _output_get_2 (`local.BeatTime`))) 1) (`local.BeatTime`))))

(fn `CheckIfDeflected`
  (returns (IsDeflected :type Boolean))
  (return (`self.IsDeflected`)))

(fn `UserConstructionScript`)